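; Game mode Blueprint that holds the day/night state and starts the game in day.
; On BeginPlay it shows and enables collision on actors tagged DayOnly, and does the reverse for NightOnly actors in a loop nested inside the DayOnly loop.
; ToggleDayNight flips IsDay and broadcasts OnDayNightChanged with the new value, without updating the tagged actors itself.
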(event EventBeginPlay
  (Variables|Default|SetisDay true)
  (bind _outactors (Actor|GetAllActorswithTag "DayOnly"))
  (for _array_element _outactors
    (Rendering|SetActorHiddenInGame _array_element false)
    (Collision|SetActorEnableCollision _array_element true)
    (bind _outactors_2 (Actor|GetAllActorswithTag "NightOnly"))
    (for _array_element_2 _outactors_2
      (Rendering|SetActorHiddenInGame _array_element_2 true)
      (Collision|SetActorEnableCollision _array_element_2 false))))

(fn ConstructionScript)

(fn ToggleDayNight
  (bind _output_get (Variables|Default|SetisDay (not (Variables|Default|GetisDay))))
  (Default|CallOnDayNightChanged _output_get))